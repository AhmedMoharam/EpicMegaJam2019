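; Game state for an elemental soul level, tracking pickups and deciding when the level is won.
; On BeginPlay it caches the game instance and player, creates the HUD and fetches the required Earth count.
; Pickup functions drive the character's forms and catalyst, while state and hint functions update the HUD.
; Having enough Earth inside the end trigger calls the end cutscene; the next-level call is disconnected.
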(event `self.ReceiveBeginPlay`
  (`|ExecutionSequence`
    (:`then_0`
      (bind _assoul_game_instanse (cast `/Game/Blueprints/Soul_GameInstanse` (`GameplayStatics.GetGameInstance`)))
      (set `self.SoulGameInstance` _assoul_game_instanse)
      (bind _assoul_bp (cast `/Game/Character/Soul_BP` (`GameplayStatics.GetPlayerCharacter` 0)))
      (set `self.Soul_character_ref` _assoul_bp))
    (:`then_1`
      (bind _returnvalue (`|CreateWidget` "/Game/UI/GamePlayUI.GamePlayUI_C"))
      (bind _output_get (set `self.GameUiRef` _returnvalue))
      (`UserWidget.AddToViewport` _output_get 0))
    (:`then_2`
      (bind _neededearthcount (`/Game/Blueprints/Soul_GameInstanse.getNeededEarthCount` (`self.SoulGameInstance`)))
      (bind _output_get_2 (set `self.NeededEarthCount` _neededearthcount))
      (set `/Game/UI/GamePlayUI.TotalEarthNeeded` _output_get_2 (`self.GameUiRef`)))))

(fn `AddHintMessage`
  (params (Message :type Text))
  (set `/Game/UI/GamePlayUI.HintMessage` Message (`self.GameUiRef`)))

(fn `AirAcquired`
  (bind _soul_character_ref (`self.Soul_character_ref`))
  (`BlueprintSetLibrary.Set_Add` (`/Game/Character/Soul_BP.OwnedElements` _soul_character_ref) "NewEnumerator3")
  (`/Game/Character/Soul_BP.TransformAir` _soul_character_ref)
  (set `/Game/UI/GamePlayUI.ElementalForm` "NewEnumerator3" (`self.GameUiRef`)))

(fn `CatalystAcquired`
  (params (CorrespondingComplexElement :type "/Game/Blueprints/Level_Objs/ComplexElementsEnum Enum" :default "NewEnumerator0"))
  (set `self.IsACatalystAcquired` true)
  (bind _output_get (set `self.CatalystEnum` CorrespondingComplexElement))
  (switch `/Game/Blueprints/Level_Objs/ComplexElementsEnum` _output_get
    (:`NewEnumerator0`
      _)
    (:`NewEnumerator1`
      _)
    (:`NewEnumerator2`
      _))
  (`/Game/Character/Soul_BP.AddOrbitingCatalyst` (`self.Soul_character_ref`)))

(fn `CatalystWasted`
  (set `self.IsACatalystAcquired` false)
  (`/Game/Character/Soul_BP.WasteCatalyst` (`self.Soul_character_ref`)))

(fn `CheckWon`
  (if (and (`self.OverlappingEndLevelTriggerVoulme`) (>= (`self.CurrnetEarthCount`) (`self.NeededEarthCount`)))
    (`self.EndCutscene`)))

(fn `ClearHintMessage`
  (set `/Game/UI/GamePlayUI.HintMessage` "" (`self.GameUiRef`)))

(fn `EarthAcquired`
  (bind _output_get (set `self.CurrnetEarthCount` (+ (`self.CurrnetEarthCount`) 1)))
  (set `/Game/UI/GamePlayUI.CollectedEarthCount` _output_get (`self.GameUiRef`))
  (`self.CheckWon`))

(fn `FireAcquired`
  (bind _soul_character_ref (`self.Soul_character_ref`))
  (`BlueprintSetLibrary.Set_Add` (`/Game/Character/Soul_BP.OwnedElements` _soul_character_ref) "NewEnumerator1")
  (`/Game/Character/Soul_BP.TransformFire` _soul_character_ref)
  (set `/Game/UI/GamePlayUI.ElementalForm` "NewEnumerator1" (`self.GameUiRef`)))

(fn `NoifyStateChange`
  (params (NewState :type "/Game/Character/SoulElementalState Enum" :default "NewEnumerator0"))
  (bind _gameuiref (`self.GameUiRef`))
  (switch `/Game/Character/SoulElementalState` NewState
    (:`NewEnumerator0`
      (set `/Game/UI/GamePlayUI.ElementalForm` "NewEnumerator0" _gameuiref))
    (:`NewEnumerator1`
      (set `/Game/UI/GamePlayUI.ElementalForm` "NewEnumerator1" _gameuiref))
    (:`NewEnumerator2`
      (set `/Game/UI/GamePlayUI.ElementalForm` "NewEnumerator2" _gameuiref))
    (:`NewEnumerator3`
      (set `/Game/UI/GamePlayUI.ElementalForm` "NewEnumerator3" _gameuiref))))

(fn `TriggeredVolumeEnd`
  (set `self.OverlappingEndLevelTriggerVoulme` false))

(fn `TriggeredVolumeStart`
  (set `self.OverlappingEndLevelTriggerVoulme` true)
  (`self.CheckWon`))

(fn `UserConstructionScript`)

(fn `WaterAcquired`
  (bind _soul_character_ref (`self.Soul_character_ref`))
  (`BlueprintSetLibrary.Set_Add` (`/Game/Character/Soul_BP.OwnedElements` _soul_character_ref) "NewEnumerator2")
  (`/Game/Character/Soul_BP.TrasformWater` _soul_character_ref)
  (set `/Game/UI/GamePlayUI.ElementalForm` "NewEnumerator2" (`self.GameUiRef`)))