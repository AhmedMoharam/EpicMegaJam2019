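; Level puzzle actor that teleports an overlapping Soul_BP to a destination chosen by the trigger volume it last entered.
; The destination starts at a default target point, and each of five trigger volumes switches it to its paired target point.
; Entering the teleportation volume moves the Soul to that point's X and Y, with Z and rotation read through a helper on the Soul.
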(event `self.ReceiveBeginPlay`
  (set `self.TeleportationLocation` (`SceneComponent.K2_GetComponentLocation` (`self.DefaultTargetPoint`))))

(event `self.TeleportationVolume.OnComponentBeginOverlap`
  (params (OverlappedComponent :type "PrimitiveComponent Object Reference") (OtherActor :type "Actor Object Reference") (OtherComp :type "PrimitiveComponent Object Reference") (OtherBodyIndex :type Integer) (bFromSweep :type Boolean) (SweepResult :type "HitResult Structure (by ref)"))
  (bind (_teleportationlocation_x _teleportationlocation_y) (`KismetMathLibrary.BreakVector` (`self.TeleportationLocation`)))
  (bind _assoul_bp (cast `/Game/Character/Soul_BP` OtherActor))
  (bind _returnvalue (`self.GetTransform` _assoul_bp))
  (`self.K2_TeleportTo` _assoul_bp (`KismetMathLibrary.MakeVector` _teleportationlocation_x _teleportationlocation_y (.z (.location _returnvalue))) (.rotation _returnvalue)))

(event `self.TriggerVolume1.OnComponentBeginOverlap`
  (params (OverlappedComponent :type "PrimitiveComponent Object Reference") (OtherActor :type "Actor Object Reference") (OtherComp :type "PrimitiveComponent Object Reference") (OtherBodyIndex :type Integer) (bFromSweep :type Boolean) (SweepResult :type "HitResult Structure (by ref)"))
  (cast `/Game/Character/Soul_BP` OtherActor)
  (set `self.TeleportationLocation` (`SceneComponent.K2_GetComponentLocation` (`self.TargetPoint1`))))

(event `self.TriggerVolume2.OnComponentBeginOverlap`
  (params (OverlappedComponent :type "PrimitiveComponent Object Reference") (OtherActor :type "Actor Object Reference") (OtherComp :type "PrimitiveComponent Object Reference") (OtherBodyIndex :type Integer) (bFromSweep :type Boolean) (SweepResult :type "HitResult Structure (by ref)"))
  (cast `/Game/Character/Soul_BP` OtherActor)
  (set `self.TeleportationLocation` (`SceneComponent.K2_GetComponentLocation` (`self.TargetPoint2`))))

(event `self.TriggerVolume3.OnComponentBeginOverlap`
  (params (OverlappedComponent :type "PrimitiveComponent Object Reference") (OtherActor :type "Actor Object Reference") (OtherComp :type "PrimitiveComponent Object Reference") (OtherBodyIndex :type Integer) (bFromSweep :type Boolean) (SweepResult :type "HitResult Structure (by ref)"))
  (cast `/Game/Character/Soul_BP` OtherActor)
  (set `self.TeleportationLocation` (`SceneComponent.K2_GetComponentLocation` (`self.TargetPoint3`))))

(event `self.TriggerVolume4.OnComponentBeginOverlap`
  (params (OverlappedComponent :type "PrimitiveComponent Object Reference") (OtherActor :type "Actor Object Reference") (OtherComp :type "PrimitiveComponent Object Reference") (OtherBodyIndex :type Integer) (bFromSweep :type Boolean) (SweepResult :type "HitResult Structure (by ref)"))
  (cast `/Game/Character/Soul_BP` OtherActor)
  (set `self.TeleportationLocation` (`SceneComponent.K2_GetComponentLocation` (`self.TargetPoint4`))))

(event `self.TriggerVolume5.OnComponentBeginOverlap`
  (params (OverlappedComponent :type "PrimitiveComponent Object Reference") (OtherActor :type "Actor Object Reference") (OtherComp :type "PrimitiveComponent Object Reference") (OtherBodyIndex :type Integer) (bFromSweep :type Boolean) (SweepResult :type "HitResult Structure (by ref)"))
  (cast `/Game/Character/Soul_BP` OtherActor)
  (set `self.TeleportationLocation` (`SceneComponent.K2_GetComponentLocation` (`self.TargetPoint5`))))

(fn `UserConstructionScript`)