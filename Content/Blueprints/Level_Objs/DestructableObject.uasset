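; A destructible wall actor that disappears when destroyed and respawns after a set delay.
; Destroy hides the DestructableWall component and disables its collision behind a DoOnce, then starts a SpawnTime timer.
; Spawn restores visibility and the collision mode cached at BeginPlay, then resets the DoOnce.
; The actor enables input from player 0, so pressing F also triggers Destroy, with no proximity check.
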(event `self.ReceiveBeginPlay`
  (set `self.Collision Enabled` (`PrimitiveComponent.GetCollisionEnabled` (`self.DestructableWall`)))
  (`self.EnableInput` (`GameplayStatics.GetPlayerController` 0)))

(event `Key|F`
  (params (Key :type "Key Structure"))
  (:`Pressed`
    (`self.Destroy`)))

(event `Destroy`
  (`/Engine/EditorBlueprintResources/StandardMacros.DoOnce` false :!label _label
    (:`Completed`
      (bind _returnvalue (`KismetSystemLibrary.K2_SetTimerDelegate` (delegate `Spawn`) (`self.SpawnTime`)))
      (set `self.SpawnTimer` _returnvalue)
      (`SceneComponent.SetVisibility` (`self.DestructableWall`) false false)
      (`PrimitiveComponent.SetCollisionEnabled` (`self.DestructableWall`) "NoCollision"))))

(event `Spawn`
  (`SceneComponent.SetVisibility` (`self.DestructableWall`) true false)
  (`PrimitiveComponent.SetCollisionEnabled` (`self.DestructableWall`) (`self.Collision Enabled`))
  (`KismetSystemLibrary.K2_ClearAndInvalidateTimerHandle` (`self.SpawnTimer`))
  (goto _label :!via `Reset`))

(fn `UserConstructionScript`)