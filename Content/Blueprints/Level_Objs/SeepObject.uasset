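; SeepObject is an interactable level object that carries the player's Soul_BP along a spline when it is in a specific elemental state.
; Box overlap caches the soul and enables input, and leaving disables it.
; Pressing E in the matching state runs a timeline scaled by Duration.
; The timeline moves the soul along the full spline length, preserving its initial offset from the spline start, without sweeping.
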(event `MoveOverSpline`
  (`TimelineComponent.SetPlayRate` (`self.SplineTimeline`) (/ 1.0 (`self.Duration`)))
  (set `self.splineOffsetvec` (- (`SplineComponent.GetLocationAtDistanceAlongSpline` (`self.Spline`) 0.0 "World") (`SceneComponent.K2_GetComponentLocation` (`Actor.RootComponent` (`self.Soul_BP`)))))
  (bind (_direction _value) (`Timeline|SplineTimeline` :!via `PlayFromStart`)
    (:`Update`
      (`SceneComponent.K2_SetWorldLocation` (`Actor.RootComponent` (`self.Soul_BP`)) (- (`SplineComponent.GetLocationAtDistanceAlongSpline` (`self.Spline`) (`KismetMathLibrary.Lerp` 0.0 (`SplineComponent.GetSplineLength` (`self.Spline`)) _value) "World") (`self.splineOffsetvec`)) false false))))

(event `self.Box.OnComponentBeginOverlap`
  (params (OverlappedComponent :type "PrimitiveComponent Object Reference") (OtherActor :type "Actor Object Reference") (OtherComp :type "PrimitiveComponent Object Reference") (OtherBodyIndex :type Integer) (bFromSweep :type Boolean) (SweepResult :type "HitResult Structure (by ref)"))
  (bind _assoul_bp (cast `/Game/Character/Soul_BP` OtherActor))
  (set `self.Soul_BP` _assoul_bp)
  (`self.EnableInput` (`GameplayStatics.GetPlayerController` 0)))

(event `self.Box.OnComponentEndOverlap`
  (params (OverlappedComponent :type "PrimitiveComponent Object Reference") (OtherActor :type "Actor Object Reference") (OtherComp :type "PrimitiveComponent Object Reference") (OtherBodyIndex :type Integer))
  (cast `/Game/Character/Soul_BP` OtherActor)
  (`self.DisableInput` (`GameplayStatics.GetPlayerController` 0)))

(event `Key|E`
  (params (Key :type "Key Structure"))
  (:`Pressed`
    (if (`|EnumEquality` (`/Game/Character/Soul_BP.ElementalState` (`self.Soul_BP`)) "NewEnumerator2")
      (`self.MoveOverSpline`))))

(fn `UserConstructionScript`)