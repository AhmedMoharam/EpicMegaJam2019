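; ScaleableObject is a level object whose cube the player can rescale once by pressing E while a Soul_BP is inside its trigger box.
; Box overlaps enable and disable the object's input, and a DoOnce on E calls ReScale.
; ReScale captures the cube's world scale, then a timeline lerps each axis toward that scale times its per-axis multiplier, with play rate derived from Duration.
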(event `ReScale`
  (bind _initialxscale (`self.initialXScale`))
  (bind _initialyscale (`self.initialYScale`))
  (bind _initialzscale (`self.initialZScale`))
  (bind (_returnvalue_x _returnvalue_y _returnvalue_z) (`KismetMathLibrary.BreakVector` (`SceneComponent.K2_GetComponentScale` (`self.Cube`))))
  (`KismetSystemLibrary.PrintString` "Re-Scaling")
  (`TimelineComponent.SetPlayRate` (`self.ScalingTimeline`) (/ 1.0 (`self.Duration`)))
  (set `self.initialXScale` _returnvalue_x)
  (set `self.initialYScale` _returnvalue_y)
  (set `self.initialZScale` _returnvalue_z)
  (bind (_direction _value) (`Timeline|ScalingTimeline`)
    (:`Update`
      (`SceneComponent.SetWorldScale3D` (`self.Cube`) (`KismetMathLibrary.MakeVector` (`KismetMathLibrary.Lerp` _initialxscale (* _initialxscale (`self.ScaleX`)) _value) (`KismetMathLibrary.Lerp` _initialyscale (* _initialyscale (`self.ScaleY`)) _value) (`KismetMathLibrary.Lerp` _initialzscale (* _initialzscale (`self.ScaleZ`)) _value))))))

(event `self.Box.OnComponentBeginOverlap`
  (params (OverlappedComponent :type "PrimitiveComponent Object Reference") (OtherActor :type "Actor Object Reference") (OtherComp :type "PrimitiveComponent Object Reference") (OtherBodyIndex :type Integer) (bFromSweep :type Boolean) (SweepResult :type "HitResult Structure (by ref)"))
  (cast `/Game/Character/Soul_BP` OtherActor)
  (`self.EnableInput` (`GameplayStatics.GetPlayerController` 0)))

(event `self.Box.OnComponentEndOverlap`
  (params (OverlappedComponent :type "PrimitiveComponent Object Reference") (OtherActor :type "Actor Object Reference") (OtherComp :type "PrimitiveComponent Object Reference") (OtherBodyIndex :type Integer))
  (cast `/Game/Character/Soul_BP` OtherActor)
  (`self.DisableInput` (`GameplayStatics.GetPlayerController` 0)))

(event `Key|E`
  (params (Key :type "Key Structure"))
  (:`Pressed`
    (`/Engine/EditorBlueprintResources/StandardMacros.DoOnce` false
      (:`Completed`
        (`self.ReScale`)))))

(fn `UserConstructionScript`)