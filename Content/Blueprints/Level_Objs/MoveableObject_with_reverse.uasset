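; Interactable level object that travels along a spline when the player presses E, then returns after a delay.
; A box trigger enables input while a Soul_BP overlaps it and disables it on exit.
; A timeline, rate-scaled by Duration, drives the object over the spline's length, preserving its offset from the spline start captured on each press.
; A timer started on the press reverses the timeline after WaitingTimeBeforeReverse.
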(event `self.ReceiveBeginPlay`)

(event `MoveOverSpline`
  (`TimelineComponent.SetPlayRate` (`self.SplineTimeline`) (/ 1.0 (`self.Duration`)))
  (set `self.splineOffsetvec` (- (`SplineComponent.GetLocationAtDistanceAlongSpline` (`self.Spline`) 0.0 "World") (`SceneComponent.K2_GetComponentLocation` (`self.Object`))))
  (bind (_direction _value) (`Timeline|SplineTimeline` :!label _label)
    (:`Update`
      (`SceneComponent.K2_SetWorldLocation` (`self.Object`) (- (`SplineComponent.GetLocationAtDistanceAlongSpline` (`self.Spline`) (`KismetMathLibrary.Lerp` 0.0 (`SplineComponent.GetSplineLength` (`self.Spline`)) _value) "World") (`self.splineOffsetvec`)) false false))))

(event `self.Box.OnComponentBeginOverlap`
  (params (OverlappedComponent :type "PrimitiveComponent Object Reference") (OtherActor :type "Actor Object Reference") (OtherComp :type "PrimitiveComponent Object Reference") (OtherBodyIndex :type Integer) (bFromSweep :type Boolean) (SweepResult :type "HitResult Structure (by ref)"))
  (cast `/Game/Character/Soul_BP` OtherActor)
  (`self.EnableInput` (`GameplayStatics.GetPlayerController` 0)))

(event `self.Box.OnComponentEndOverlap`
  (params (OverlappedComponent :type "PrimitiveComponent Object Reference") (OtherActor :type "Actor Object Reference") (OtherComp :type "PrimitiveComponent Object Reference") (OtherBodyIndex :type Integer))
  (cast `/Game/Character/Soul_BP` OtherActor)
  (`self.DisableInput` (`GameplayStatics.GetPlayerController` 0)))

(event `Key|E`
  (params (Key :type "Key Structure"))
  (:`Pressed`
    (`self.MoveOverSpline`)
    (bind _returnvalue (`KismetSystemLibrary.K2_SetTimerDelegate` (delegate `reverse`) (`self.WaitingTimeBeforeReverse`)))
    (set `self.WaitingTimerRefernce` _returnvalue)))

(event `reverse`
  (goto _label :!via `Reverse`))

(fn `UserConstructionScript`)