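; Pressure-panel door that slides sideways along its local Y axis while a Soul_BP or MoveableObject actor rests on the panel.
; A looping timer polls the trigger's overlaps to set IsActivated, with paired gates passing color updates to the panel materials when the state flips.
; Tick moves the door toward its open or closed limit at a speed from Distance over Time, unless IsTrapped halts it.
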(event `self.ReceiveBeginPlay`
  ;[1 1 1] Init
  (`KismetSystemLibrary.K2_SetTimerDelegate` (delegate `TimerTick`) 0.1 true)
  (set `self.InitialLocation` (`SceneComponent.K2_GetComponentLocation` (`self.Door`))))

(event `TimerTick`
  ;[1 1 1] Init
  (`self.CubeCheck`))

(event `self.ReceiveTick`
  (params (DeltaSeconds :type "Float (single-precision)"))
  ;[1 1 1] Door
  (set `self.DeltaSeconds` DeltaSeconds)
  (set `self.atTheStart` (<= (`self.GetInitialY`) (`self.GetCurrentY`)))
  (set `self.atTheEnd` (>= (- (`self.GetInitialY`) (`self.GetCurrentY`)) (`self.Distance`)))
  (if (`self.isTrapped`)
    _
    (elif (`self.isActivated`)
      (if (not (`self.atTheEnd`))
        (`self.Raise`))
      (elif (not (`self.atTheStart`))
        (`self.Lower`)))))

(event `CubeCheck`
  (bind _overlappingactors (`PrimitiveComponent.GetOverlappingActors` (`self.PanelTrigger`) null))
  ;[1 1 1] Panel
  ;;[1 1 1] Checking for Small Cube
  (if (<= (`KismetArrayLibrary.Array_Length` _overlappingactors) 0)
    (set `self.isActivated` false)
    (`/Engine/EditorBlueprintResources/StandardMacros.Gate` false :!label _label
      (:`Exit`
        (`|ExecutionSequence`
          (:`then_0`
            (goto _label :!via `Toggle`))
          (:`then_1`
            (`self.ColorUpdate` :!label _label_2))
          (:`then_2`
            (goto _label_3 :!via `Toggle`)))))
    (else
      (for _array_element _overlappingactors
        (bind _returnvalue (`GameplayStatics.GetObjectClass` _array_element))
        (if (or (== _returnvalue "/Game/Character/Soul_BP.Soul_BP_C") (== _returnvalue "/Game/Blueprints/Level_Objs/MoveableObject.MoveableObject_C"))
          (set `self.isActivated` true)
          (`/Engine/EditorBlueprintResources/StandardMacros.Gate` true :!label _label_3
            (:`Exit`
              (`|ExecutionSequence`
                (:`then_0`
                  (goto _label :!via `Toggle`))
                (:`then_1`
                  (goto _label_2))
                (:`then_2`
                  (goto _label_3 :!via `Toggle`))))))))))

(event `ColorUpdate`
  (bind _smallpanel (`self.SmallPanel`))
  (bind _smallpanel_2 (`self.SmallPanel`))
  (bind _returnvalue (`KismetMathLibrary.Conv_LinearColorToVector` (`KismetMathLibrary.MakeColor` 255.0 200.0)))
  ;[1 1 1] Panel
  ;;[1 1 1] Updating Color
  (if (`self.isActivated`)
    (`MeshComponent.SetVectorParameterValueOnMaterials` _smallpanel_2 "PrimaryColor" _returnvalue)
    (`MeshComponent.SetVectorParameterValueOnMaterials` _smallpanel_2 "SecondaryColor" _returnvalue)
    (else
      (`MeshComponent.SetVectorParameterValueOnMaterials` _smallpanel "PrimaryColor" (`KismetMathLibrary.Conv_LinearColorToVector` (`KismetMathLibrary.MakeColor` 0.0)))
      (`MeshComponent.SetVectorParameterValueOnMaterials` _smallpanel "SecondaryColor" (`KismetMathLibrary.Conv_LinearColorToVector` (`KismetMathLibrary.MakeColor` 0.0 0.0 0.0 2.0))))))

(fn `UserConstructionScript`)